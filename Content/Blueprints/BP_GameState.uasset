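; Game state Blueprint that runs a timed match, from the in-game HUD to the end screen.
; BeginPlay shows the in-game widget, sets game-only input, hides the cursor and starts a looping one-second timer calling DecreaseTime.
; DecreaseTime counts GameTime down, then clears the timer, removes the HUD, pauses the game and shows the end screen with UI-only input and a visible cursor.
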(event `self.ReceiveBeginPlay`
  (bind _returnvalue (`GameplayStatics.GetPlayerController` 0))
  ;[1 1 1] BeginPlay
  (`|ExecutionSequence`
    (:`then_0`
      ;;[1 1 1] Create In Game widget
      (bind _returnvalue_2 (`|CreateWidget` "/Game/UI/WBP_InGame_Screen.WBP_InGame_Screen_C"))
      (bind _output_get (set `self.InGameRef` _returnvalue_2))
      (`UserWidget.AddToViewport` _output_get 0)
      (`WidgetBlueprintLibrary.SetInputMode_GameOnly` _returnvalue)
      (set `PlayerController.bShowMouseCursor` false _returnvalue))
    (:`then_1`
      ;;[0 1 0.9773] Start Countdown
      (`self.StartCountdown`))))

(event `StartCountdown`
  ;[1 1 1] StartCountDown Event
  (bind _returnvalue (`KismetSystemLibrary.K2_SetTimer` null "DecreaseTime" 1.0 true))
  (set `self.TimerHadle` _returnvalue))

(fn `DecreaseTime`
  (bind _returnvalue (`GameplayStatics.GetPlayerController` 0))
  ;[1 1 1] Calculation Gameplay Timer
  (if (> (`self.GameTime`) 0.0)
    (set `self.GameTime` (- (`self.GameTime`) 1.0))
    (else
      (`KismetSystemLibrary.K2_ClearAndInvalidateTimerHandle` (`self.TimerHadle`))
      ;[1 1 1] Remove From parent
      (`Widget.RemoveFromParent` (`self.InGameRef`))
      (`GameplayStatics.SetGamePaused` true)
      ;[1 1 1] Create End Screen widget
      (bind _returnvalue_2 (`|CreateWidget` "/Game/UI/WBP_EndScreen.WBP_EndScreen_C"))
      (`UserWidget.AddToViewport` _returnvalue_2 0)
      (`WidgetBlueprintLibrary.SetInputMode_UIOnlyEx` _returnvalue _returnvalue_2)
      (set `PlayerController.bShowMouseCursor` true _returnvalue))))

(fn `UserConstructionScript`)