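; BP_Range_Target is a range target that falls over when FallFunction is called, then stands back up after a random few seconds.
; Timelines lerp the root's roll between upright and flat, while the cube's collision is disabled on falling and restored on rising.
; The fall timeline sets the looping rise timer on every update, and the rise timeline clears it as it plays.
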(event `Fall Function`
  ;[1 1 1] FallFunction
  (`PrimitiveComponent.SetCollisionEnabled` (`self.Cube`) "NoCollision")
  (bind (_direction _delta) (`Timeline|Timeline` :!via `PlayFromStart`)
    (:`Update`
      (`SceneComponent.K2_SetRelativeRotation` (`self.DefaultSceneRoot`) (`KismetMathLibrary.MakeRotator` (`KismetMathLibrary.Lerp` 0.0 90.0 _delta)) false false)
      ;[1 1 1] Timer Event
      (bind _returnvalue (`KismetSystemLibrary.K2_SetTimerDelegate` (delegate `Rise Function`) (`KismetMathLibrary.RandomFloatInRange` 2.0 7.0) true))
      (set `self.TimerHandle` _returnvalue))))

(event `Rise Function`
  ;[1 1 1] Rise Function
  (`PrimitiveComponent.SetCollisionEnabled` (`self.Cube`) "QueryAndPhysics")
  (bind (_direction _delta) (`Timeline|Timeline_0` :!via `PlayFromStart`)
    (:`Update`
      (`SceneComponent.K2_SetRelativeRotation` (`self.DefaultSceneRoot`) (`KismetMathLibrary.MakeRotator` (`KismetMathLibrary.Lerp` 90.0 0.0 _delta)) false false)
      (`KismetSystemLibrary.K2_ClearAndInvalidateTimerHandle` (`self.TimerHandle`)))))

(fn `UserConstructionScript`)